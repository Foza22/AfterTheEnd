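; Player inventory component that extends a parent inventory component and keeps the player's item slot display in sync with item changes.
; Slot drops from the player inventory or hotbar are forwarded to the source container's TransferItem, targeting this component.
; Adding or removing an item runs the parent logic, then messages the owner's controller to update or reset that slot.
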(event EventBeginPlay
  (|CallParentFunction) ; This node is disabled and will not be called.\nDrag off pins to build functionality.
)

(event EventTick
  (params (DeltaSeconds :type Float%20%28single-precision%29))
  (|CallParentFunction DeltaSeconds) ; This node is disabled and will not be called.\nDrag off pins to build functionality.
)

(fn HandleSlotDrop
  (params (From%20Container :type BP%20Items%20Container%20Component%20Object%20Reference) (From%20Index :type Integer) (ToIndex :type Integer))
  (LocalVariables|SetLocalFromContainer From%20Container)
  (LocalVariables|SetLocalFromIndex From%20Index)
  (LocalVariables|SetLocalToIndex ToIndex)
  (switch Utilities|FlowControl|Switch|SwitchonE_ContainerType (Variables|/Game/InventorySystem/Inventory/BP_ItemsContainerComponent.BP_ItemsContainerComponent_C|GetContainerType (LocalVariables|GetLocalFromContainer))
    (:NewEnumerator0
      _)
    (:NewEnumerator1
      _))
  (Default|TransferItem (LocalVariables|GetLocalFromContainer) self (LocalVariables|GetLocalToIndex) (LocalVariables|GetLocalFromIndex))
  (return))

(fn AddItemtoIndex
  (params (Item :type S%20Item%20Info%20Structure) (ToIndex :type Integer) (FromIndex :type Integer))
  (bind _bsuccess (|CallParentFunction Item ToIndex FromIndex))
  (bind _controllerref (Class|BPICharacter|GetControllerfromChar(Message) (Components|GetOwner)))
  (Default|UpdateItemSlot _controllerref (Variables|Default|GetContainerType) ToIndex (CallFunction|GetItematIndex ToIndex))
  (return _bsuccess))

(fn RemoveItematIndex
  (params (Index :type Integer))
  (bind _bsuccess (|CallParentFunction Index))
  (bind _controllerref (Class|BPICharacter|GetControllerfromChar(Message) (Components|GetOwner)))
  (Default|ResetItemSlot _controllerref (Variables|Default|GetContainerType) Index)
  (return _bsuccess))