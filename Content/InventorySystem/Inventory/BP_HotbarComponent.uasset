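; Hotbar component for the inventory system that reports what occupies a given hotbar slot.
; CheckHotbar reads the Items entry at an index, treats an ItemID of zero as empty, and returns whether the slot is filled along with its item type.
; The event graph holds only disabled BeginPlay and Tick stubs, so the component runs no logic of its own outside that lookup.
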(event EventBeginPlay
  (|CallParentFunction) ; This node is disabled and will not be called.\nDrag off pins to build functionality.
)

(event EventTick
  (params (DeltaSeconds :type Float%20%28single-precision%29))
  (|CallParentFunction DeltaSeconds) ; This node is disabled and will not be called.\nDrag off pins to build functionality.
)

(fn CheckHotbar
  (params (Index :type Integer))
  (bind _items (Variables|Default|GetItems))
  (bind _output (Utilities|Array|Get(acopy) _items Index))
  (bind (_itemid _itemquantity _itemicon _itemname _itemdesc _itemdamage _itemrarity _itemcurhp _itemmaxhp _isstackable_ _stacksize _itemtype) (Utilities|Struct|BreakS_ItemInfo _output))
  (if (== _itemid 0)
    (return false "NewEnumerator0")
    (else
      (return true _itemtype))))