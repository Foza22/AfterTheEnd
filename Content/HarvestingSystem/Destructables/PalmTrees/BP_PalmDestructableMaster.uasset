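; Master Blueprint for destructible palm trees in the harvesting system, dissolving the palm away shortly after it spawns.
; After BeginPlay runs the parent logic and a fixed delay, it creates dynamic material instances for the static mesh's six palm material slots.
; A timeline drives the Dissolve scalar on all six, then hides the mesh on completion without destroying the actor.
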(event EventBeginPlay
  (bind _staticmesh (Variables|Default|GetStaticMesh))
  (|CallParentFunction)
  (Utilities|FlowControl|Delay 1e+01)
  (bind _returnvalue (Rendering|Material|CreateDynamicMaterialInstance _staticmesh 0 "/Game/Assets/PalmTrees/Materials/MI_Palm01.MI_Palm01" "None" :!class /Script/Engine.PrimitiveComponent))
  (Variables|Default|SetMat0 _returnvalue)
  (bind _returnvalue_2 (Rendering|Material|CreateDynamicMaterialInstance _staticmesh 1 "/Game/Assets/PalmTrees/Materials/MI_Palm02.MI_Palm02" "None" :!class /Script/Engine.PrimitiveComponent))
  (Variables|Default|SetMat1 _returnvalue_2)
  (bind _returnvalue_3 (Rendering|Material|CreateDynamicMaterialInstance _staticmesh 2 "/Game/Assets/PalmTrees/Materials/MI_Palm03.MI_Palm03" "None" :!class /Script/Engine.PrimitiveComponent))
  (Variables|Default|SetMat2 _returnvalue_3)
  (bind _returnvalue_4 (Rendering|Material|CreateDynamicMaterialInstance _staticmesh 3 "/Game/Assets/PalmTrees/Materials/MI_Palm03.MI_Palm03" "None" :!class /Script/Engine.PrimitiveComponent))
  (Variables|Default|SetMat3 _returnvalue_4)
  (bind _returnvalue_5 (Rendering|Material|CreateDynamicMaterialInstance _staticmesh 4 "/Game/Assets/PalmTrees/Materials/MI_Palm_Leaf.MI_Palm_Leaf" "None" :!class /Script/Engine.PrimitiveComponent))
  (Variables|Default|SetMat4 _returnvalue_5)
  (bind _returnvalue_6 (Rendering|Material|CreateDynamicMaterialInstance _staticmesh 5 "/Game/Assets/PalmTrees/Materials/MI_Palm04.MI_Palm04" "None" :!class /Script/Engine.PrimitiveComponent))
  (Variables|Default|SetMat5 _returnvalue_6)
  (bind _newtrack_0 (Timeline|FadeAwayTimelime PlayFromStart)
    (:Update
      (Rendering|Material|SetScalarParameterValue (Variables|Default|GetMat0) "Dissolve" _newtrack_0 :!class /Script/Engine.MaterialInstanceDynamic))
    (:Finished
      (Rendering|SetVisibility (Variables|Default|GetStaticMesh) false false))))

(fn ConstructionScript
  (|CallParentFunction))