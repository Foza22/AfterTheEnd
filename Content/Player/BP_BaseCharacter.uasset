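; Base player character that handles hotbar equipping, item use, inventory slot drops, the invite-list HUD and a debug hatchet spawn.
; Number keys 1-8 call HotbarOnServer, which either removes the held item or spawns the slot's equipable.
; Equipping attaches separate third-person (multicast) and first-person actors to their meshes.
; Attacks forward to the third-person item, which also receives montage notify and completion messages.
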(event Custom|OnSlotDropOnServer
  (params (TargetContainer :type E_ContainerType%20Enum :default "NewEnumerator0") (FromContainer :type E_ContainerType%20Enum :default "NewEnumerator0") (FromIndex :type Integer) (ToIndex :type Integer) (ArmorType :type E_ArmorType%20Enum :default "NewEnumerator0"))
  (Default|OnSlotDrop (Utilities|Select :Index TargetContainer :NewEnumerator0 (Variables|Default|GetPlayerInventoryComponent) :NewEnumerator1 0 :NewEnumerator2 0 :NewEnumerator3 0) (Utilities|Select :Index FromContainer :NewEnumerator0 (Variables|Default|GetPlayerInventoryComponent) :NewEnumerator1 0 :NewEnumerator2 0 :NewEnumerator3 0) FromIndex ToIndex))

(event Custom|HotbarOnServer
  (params (Index :type Integer))
  ;[1 1 1] EquipWeapon
  (CallFunction|UseHotbar Index))

(event Custom|SpawnEquipable_TP
  (params (Class :type Actor%20Class%20Reference) (ItemInfo :type S%20Item%20Info%20Structure) (EquippedIndex :type Integer))
  ;[1 1 1] EquipWeapon
  (Variables|Default|SetEquipped%20Index EquippedIndex)
  (bind _returnvalue (Game|SpawnActorfromClass Class (Math|Transform|MakeTransform "0, 0, 0" "0, 0, 0" "1.000000,1.000000,1.000000") "Undefined" 0 0))
  (bind _output_get (Variables|Default|SetTP_EquippedItem _returnvalue))
  (Actor|SetOwner _output_get self)
  (bind _equipableref (Class|BPIEquipableItem|GetEquipableRef(Message) _output_get))
  (CallFunction|MulticastWeaponEquip _equipableref (.Socketname (Utilities|Struct|BreakS_EquipableInfo (Variables|/Game/Items/BP_EquipableMaster.BP_EquipableMaster_C|GetEquipableInfo _equipableref))) (.AnimationState (Utilities|Struct|BreakS_EquipableInfo (Variables|/Game/Items/BP_EquipableMaster.BP_EquipableMaster_C|GetEquipableInfo _equipableref))))
  (CallFunction|SpawnEquipableFP (.FirstPersonEquipClass (Utilities|Struct|BreakS_EquipableInfo (Variables|/Game/Items/BP_EquipableMaster.BP_EquipableMaster_C|GetEquipableInfo _equipableref))) (.Socketname (Utilities|Struct|BreakS_EquipableInfo (Variables|/Game/Items/BP_EquipableMaster.BP_EquipableMaster_C|GetEquipableInfo _equipableref)))))

(event Custom|MulticastWeaponEquip
  (params (Target :type Actor%20Object%20Reference) (SocketName :type Name) (EquippedState :type E_EquipableState%20Enum :default "NewEnumerator5"))
  ;[1 1 1] EquipWeapon
  (Utilities|IsValid Target
    (:Is%20Valid
      (bind _mesh (Variables|Character|GetMesh)
        (:then
          (Transformation|AttachComponentToComponent Target _mesh SocketName "KeepRelative" "KeepRelative" "KeepRelative" true)
          (Variables|Default|SetEquipState EquippedState))
        (:else)))))

(event Custom|SpawnEquipable_FP
  (params (Class :type Actor%20Class%20Reference) (SocketName :type Name))
  ;[1 1 1] EquipWeapon
  (bind _returnvalue (Game|SpawnActorfromClass Class (Math|Transform|MakeTransform "0, 0, 0" "0, 0, 0" "1.000000,1.000000,1.000000") "Undefined" 0 0))
  (bind _output_get (Variables|Default|SetFP_EquippedItem _returnvalue))
  (Actor|SetOwner _output_get self)
  (Transformation|AttachComponentToComponent _output_get (Variables|Default|GetFirstPersonMesh) SocketName "KeepRelative" "KeepRelative" "KeepRelative" true))

(event Custom|UnequipWeapon_TP
  ;[1 1 1] UnequipWeapon
  (Variables|Default|SetEquipState "NewEnumerator5"))

(event Custom|UnequilWeapon_FP
  ;[1 1 1] UnequipWeapon
  (Actor|DestroyActor (Variables|Default|GetFP_EquippedItem)))

(event Custom|AttackOnServer
  (bind _tp_equippeditem (Variables|Default|GetTP_EquippedItem)
    (:then
      (Class|BPIEquipableItem|UseItem(Message) _tp_equippeditem self))
    (:else)))

(event Custom|MontageMulticast
  (params (TP_Montage :type Anim%20Montage%20Object%20Reference))
  (Animation|Montage|PlayMontage (Variables|Character|GetMesh) TP_Montage
    (:OnCompleted
      (bind _tp_equippeditem (Variables|Default|GetTP_EquippedItem)
        (:then
          (Class|BPIEquipableItem|EndAnimation(Message) _tp_equippeditem))
        (:else)))
    (:OnNotifyBegin
      (bind _tp_equippeditem_2 (Variables|Default|GetTP_EquippedItem)
        (:then
          (Class|BPIEquipableItem|Notify(Message) _tp_equippeditem_2))
        (:else)))))

(event Custom|MontageOnClient
  (params (FP_Montage :type Anim%20Montage%20Object%20Reference))
  (Animation|Montage|PlayMontage (Variables|Default|GetFirstPersonMesh) FP_Montage))

(event Input|EnhancedActionEvents|EnhancedInputActionIA_OpenInviteList
  (params (ActionValue :type Boolean) (ElapsedSeconds :type Float%20%28double-precision%29) (TriggeredSeconds :type Float%20%28double-precision%29) (InputAction :type Input%20Action%20Object%20Reference :default "/Game/Input/Actions/IA_OpenInviteList.IA_OpenInviteList"))
  (:Started
    (bind _asbp_main_hud (Utilities|Casting|CastToBP_MainHUD (HUD|GetHUD (Game|GetPlayerController 0))))
    (Default|OpenInviteList _asbp_main_hud)))

(event Input|EnhancedActionEvents|EnhancedInputActionIA_DebugSpawnItem
  (params (ActionValue :type Boolean) (ElapsedSeconds :type Float%20%28double-precision%29) (TriggeredSeconds :type Float%20%28double-precision%29) (InputAction :type Input%20Action%20Object%20Reference :default "/Game/Input/Actions/IA_DebugSpawnItem.IA_DebugSpawnItem"))
  (:Started
    (bind _returnvalue (Utilities|GetDataTableRow "/Game/InventorySystem/DataTables/DT_Items.DT_Items" "StoneHatchet")
      (:then
        (Default|AddItemonServer (Variables|Default|GetHotbarComponent) _returnvalue)))))

(event Input|EnhancedActionEvents|EnhancedInputActionIA_Attack
  (params (ActionValue :type Boolean) (ElapsedSeconds :type Float%20%28double-precision%29) (TriggeredSeconds :type Float%20%28double-precision%29) (InputAction :type Input%20Action%20Object%20Reference :default "/Game/Input/Actions/IA_Attack.IA_Attack"))
  (:Started
    (CallFunction|AttackonServer)))

(event EventBeginPlay)

(event Collision|EventActorBeginOverlap
  (params (OtherActor :type Actor%20Object%20Reference)))

(event EventTick
  (params (DeltaSeconds :type Float%20%28single-precision%29)))

(event EventFPMontage
  (params (FP_Montage :type Anim%20Montage%20Object%20Reference))
  (CallFunction|MontageonClient FP_Montage))

(event EventTPMontage
  (params (TP_Montage :type Anim%20Montage%20Object%20Reference))
  (CallFunction|MontageMulticast TP_Montage))

(event Input|KeyboardEvents|1
  (params (Key :type Key%20Structure :default "None"))
  ;[1 1 1] Hotbar binding
  (:Pressed
    (CallFunction|HotbaronServer)))

(event Input|KeyboardEvents|2
  (params (Key :type Key%20Structure :default "None"))
  ;[1 1 1] Hotbar binding
  (:Pressed
    (CallFunction|HotbaronServer 1)))

(event Input|KeyboardEvents|3
  (params (Key :type Key%20Structure :default "None"))
  ;[1 1 1] Hotbar binding
  (:Pressed
    (CallFunction|HotbaronServer 2)))

(event Input|KeyboardEvents|4
  (params (Key :type Key%20Structure :default "None"))
  ;[1 1 1] Hotbar binding
  (:Pressed
    (CallFunction|HotbaronServer 3)))

(event Input|KeyboardEvents|5
  (params (Key :type Key%20Structure :default "None"))
  ;[1 1 1] Hotbar binding
  (:Pressed
    (CallFunction|HotbaronServer 4)))

(event Input|KeyboardEvents|6
  (params (Key :type Key%20Structure :default "None"))
  ;[1 1 1] Hotbar binding
  (:Pressed
    (CallFunction|HotbaronServer 5)))

(event Input|KeyboardEvents|7
  (params (Key :type Key%20Structure :default "None"))
  ;[1 1 1] Hotbar binding
  (:Pressed
    (CallFunction|HotbaronServer 6)))

(event Input|KeyboardEvents|8
  (params (Key :type Key%20Structure :default "None"))
  ;[1 1 1] Hotbar binding
  (:Pressed
    (CallFunction|HotbaronServer 7)))

(fn ConstructionScript)

(fn UseHotbar
  (params (Index :type Integer))
  (bind _output_get (Variables|Default|SetHotbarIndex Index))
  (bind (_hasiteminslot_ _itemtype) (Default|CheckHotbar (Variables|Default|GetHotbarComponent) _output_get))
  (if _hasiteminslot_
    (switch Utilities|FlowControl|Switch|SwitchonE_ItemType _itemtype
      (:NewEnumerator1
        (Variables|Default|GetTP_EquippedItem
          (:then
            (Actor|DestroyActor (Variables|Default|GetTP_EquippedItem))
            (CallFunction|UnequipWeaponTP)
            (CallFunction|UnequilWeaponFP))
          (:else
            (CallFunction|SpawnEquipableTP (.ItemClass (Utilities|Struct|BreakS_ItemInfo (Utilities|Array|Get(acopy) (Variables|/Game/InventorySystem/Inventory/BP_ItemsContainerComponent.BP_ItemsContainerComponent_C|GetItems (Variables|Default|GetHotbarComponent)) (Variables|Default|GetHotbarIndex)))) (Utilities|Array|Get(acopy) (Variables|/Game/InventorySystem/Inventory/BP_ItemsContainerComponent.BP_ItemsContainerComponent_C|GetItems (Variables|Default|GetHotbarComponent)) (Variables|Default|GetHotbarIndex)) (Variables|Default|GetHotbarIndex))))))))

(fn GetCharacterRef
  (return self))

(fn GetControllerfromChar
  (bind _controllerref (Class|BPIController|GetControllerRef(Message) (Pawn|GetController)))
  (return _controllerref))