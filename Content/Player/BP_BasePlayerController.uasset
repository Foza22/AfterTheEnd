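; Base player controller that owns the main in-game HUD and relays inventory UI changes to it.
; On BeginPlay it creates WBP_InGameMain and adds it to the viewport, and the IA_OpenInventory input toggles the inventory through InventoryOnClient.
; Slot update and reset events forward to the inventory grid widget by index after a validity check, leaving their Container argument unused.
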(event Custom|InventoryOnClient
  (Default|ToggleInventory (Variables|Default|GetMainWidgetRef)))

(event Custom|ResetItemSlot
  (params (Container :type E_ContainerType%20Enum :default "NewEnumerator0") (Index :type Integer))
  (bind _mainwidgetref (Variables|Default|GetMainWidgetRef))
  (bind _wbp_inventory (Variables|/Game/UI/WBP_InGameMain.WBP_InGameMain_C|GetWBP_Inventory _mainwidgetref))
  (bind _wbp_itemcontainergrid (Variables|/Game/UI/Inventory/WBP_Inventory.WBP_Inventory_C|GetWBP_ItemContainerGrid _wbp_inventory))
  (bind _slots (Variables|/Game/UI/Inventory/WBP_ItemContainerGrid.WBP_ItemContainerGrid_C|GetSlots _wbp_itemcontainergrid))
  (bind _output (Utilities|Array|Get(acopy) _slots Index))
  (Utilities|IsValid _output
    (:Is%20Valid
      (Default|ResetSlot _output))))

(event Custom|UpdateItemSlot
  (params (Container :type E_ContainerType%20Enum :default "NewEnumerator0") (Index :type Integer) (ItemInfo :type S%20Item%20Info%20Structure))
  (bind _mainwidgetref (Variables|Default|GetMainWidgetRef))
  (bind _wbp_inventory (Variables|/Game/UI/WBP_InGameMain.WBP_InGameMain_C|GetWBP_Inventory _mainwidgetref))
  (bind _wbp_itemcontainergrid (Variables|/Game/UI/Inventory/WBP_Inventory.WBP_Inventory_C|GetWBP_ItemContainerGrid _wbp_inventory))
  (bind _slots (Variables|/Game/UI/Inventory/WBP_ItemContainerGrid.WBP_ItemContainerGrid_C|GetSlots _wbp_itemcontainergrid))
  (bind _output (Utilities|Array|Get(acopy) _slots Index))
  (Utilities|IsValid _output
    (:Is%20Valid
      (Default|UpdateSlot _output ItemInfo))))

(event Input|EnhancedActionEvents|EnhancedInputActionIA_OpenInventory
  (params (ActionValue :type Boolean) (ElapsedSeconds :type Float%20%28double-precision%29) (TriggeredSeconds :type Float%20%28double-precision%29) (InputAction :type Input%20Action%20Object%20Reference :default "/Game/Input/Actions/IA_OpenInventory.IA_OpenInventory"))
  (:Started
    (CallFunction|InventoryonClient)))

(event EventBeginPlay
  (bind _returnvalue (UserInterface|CreateWidget "/Game/UI/WBP_InGameMain.WBP_InGameMain_C" (Game|GetPlayerController 0)))
  (bind _output_get (Variables|Default|SetMainWidgetRef _returnvalue))
  (UserInterface|Viewport|AddtoViewport _output_get 0))

(fn ConstructionScript)

(fn GetControllerRef
  (return self))