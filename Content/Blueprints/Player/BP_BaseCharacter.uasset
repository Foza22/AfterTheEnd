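; Base player character for a survival game, handling ground-item harvesting, hotbar equipping, tool use, inventory slot moves and crafting.
; Input calls OnServer events, with multicast and client events playing third- and first-person montages, effects and paired equippable actors on each mesh.
; Harvesting damages overlapped resources and grants randomized yields from data tables.
; Crafting consumes recipe items, then adds the result after a delay, reporting to the controller through interface messages.
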(event Custom|OnSlotDropOnServer
  (params (TargetContainer :type E_ContainerType%20Enum :default "NewEnumerator0") (FromContainer :type E_ContainerType%20Enum :default "NewEnumerator0") (FromIndex :type Integer) (ToIndex :type Integer) (ArmorType :type E_ArmorType%20Enum :default "NewEnumerator0"))
  (Default|OnSlotDrop (Utilities|Select :Index TargetContainer :NewEnumerator0 (Variables|Components|GetPlayerInventoryComponent) :NewEnumerator1 (Variables|Components|GetHotbarComponent) :NewEnumerator2 0 :NewEnumerator3 0) (Utilities|Select :Index FromContainer :NewEnumerator0 (Variables|Components|GetPlayerInventoryComponent) :NewEnumerator1 (Variables|Components|GetHotbarComponent) :NewEnumerator2 0 :NewEnumerator3 0) FromIndex ToIndex))

(event Custom|HotbarOnServer
  (params (Index :type Integer))
  ;[1 1 1] EquipWeapon
  (CallFunction|UseHotbar Index))

(event Custom|HarvestItemOnServer
  (params (Resource :type S%20Resource%20Structure%20Structure))
  ;[1 1 1] Interact
  (CallFunction|HarvestLargeItem Resource))

(event Custom|UnequipCurrentItem
  (params (Index :type Integer))
  ;[1 1 1] UnequipWeapon
  (if (== Index (Variables|Default|GetEquipped%20Index))
    (bind _tp_equippeditem (Variables|Default|GetTP_EquippedItem)
      (:then
        (Actor|DestroyActor _tp_equippeditem)
        (CallFunction|UnequipWeaponTP)
        (CallFunction|UnequipWeaponFP))
      (:else))))

(event Custom|InteractOnServer
  ;[1 1 1] Interact
  (CallFunction|OverlapGroundItems))

(event Custom|OverlapGroundItems
  ;[1 1 1] Interact
  (Variables|Default|GetTP_EquippedItem
    (:then)
    (:else
      (if (not (Variables|Default|GetIsHarvesting))
        (Variables|Default|SetIsHarvesting true)
        (bind (_outactors _returnvalue) (Collision|SphereOverlapActors (Transformation|GetActorLocation) 7e+01 (Utilities|Array|MakeArray "ObjectTypeQuery1") 0 (Utilities|Array|MakeArray self)))
        (if _returnvalue
          (CallFunction|HarvestGroundItem (Utilities|Array|Get(acopy) _outactors))
          (CallFunction|HarvestMontage)
          (else
            (Variables|Default|SetIsHarvesting false)))))))

(event Custom|HarvestMontage
  ;[1 1 1] Interact
  (Animation|Montage|PlayMontage (Variables|Character|GetMesh) "/Game/Assets/Man/Animations/Montages/AM_Pickup.AM_Pickup"
    (:then
      (CallFunction|MontageonClient "/Game/Assets/Man/Animations/Montages/AM_Pickup.AM_Pickup")
      (CallFunction|MontageMulticast "/Game/Assets/Man/Animations/Montages/AM_Pickup.AM_Pickup")
      (CallFunction|BushFXMulticast))
    (:OnCompleted
      (Variables|Default|SetIsHarvesting false))))

(event Custom|BushFXMulticast
  (bind _returnvalue (Transformation|GetActorLocation))
  ;[1 1 1] Interact
  (Effects|SpawnEmitteratLocation "/Game/Assets/Realistic_Starter_VFX_Pack_Vol2/Particles/Hit/P_BushHarvest.P_BushHarvest" _returnvalue)
  (Audio|PlaySoundatLocation "/Game/Assets/Sounds/Harvesting/BushSFX/SC_BushHarvest.SC_BushHarvest" _returnvalue "0, 0, 0" 1.0 1.0 0.0 "/Game/Assets/Sounds/Harvesting/RockSFX/ATT_Harvesting.ATT_Harvesting" 0 0 0))

(event Custom|CheckIfCanCraft
  (params (ItemName :type Name) (Container :type E_ContainerType%20Enum :default "NewEnumerator0") (TableType :type E_CraftingType%20Enum :default "NewEnumerator0"))
  ;[1 1 1] Check craft possibility
  (bind _bcancraft (CallFunction|CanCraftItem (Utilities|Text|ToText(Name) ItemName) Container TableType))
  (bind _controllerref (Class|BPIController|GetControllerRef(Message) (Pawn|GetController)))
  (Default|UpdateCraftStatus _controllerref _bcancraft))

(event Custom|CraftItemOnServer
  (params (ItemName :type Text) (Container :type E_ContainerType%20Enum :default "NewEnumerator0") (TableType :type E_CraftingType%20Enum :default "NewEnumerator0"))
  ;[1 1 1] Craft item
  (if (not (Variables|Default|GetIsCrafting))
    (Variables|Default|SetIsCrafting true)
    (bind (_bcancraft _crafteditemname _containerout) (CallFunction|CraftItem ItemName Container TableType))
    (if _bcancraft
      (Utilities|FlowControl|Delay 3.0)
      (CallFunction|AddCraftedItem _crafteditemname _containerout)
      (Variables|Default|SetIsCrafting false)
      (else
        (Variables|Default|SetIsCrafting false)))))

(event Custom|SpawnEquipable_TP
  (params (Class :type Actor%20Class%20Reference) (ItemInfo :type S%20Item%20Info%20Structure) (EquippedIndex :type Integer))
  ;[1 1 1] EquipWeapon
  (Variables|Default|SetEquipped%20Index EquippedIndex)
  (bind _returnvalue (Game|SpawnActorfromClass Class (Math|Transform|MakeTransform "0, 0, 0" "0, 0, 0" "1.000000,1.000000,1.000000") "Undefined" 0 0))
  (bind _output_get (Variables|Default|SetTP_EquippedItem _returnvalue))
  (Actor|SetOwner _output_get self)
  (bind _equipableref (Class|BPIEquipableItem|GetEquipableRef(Message) _output_get))
  (CallFunction|MulticastWeaponEquip _equipableref (.Socketname (Utilities|Struct|BreakS_EquipableInfo (Variables|/Game/Blueprints/Items/BP_EquipableMaster.BP_EquipableMaster_C|GetEquipableInfo _equipableref))) (.AnimationState (Utilities|Struct|BreakS_EquipableInfo (Variables|/Game/Blueprints/Items/BP_EquipableMaster.BP_EquipableMaster_C|GetEquipableInfo _equipableref))))
  (CallFunction|SpawnEquipableFP (.FirstPersonEquipClass (Utilities|Struct|BreakS_EquipableInfo (Variables|/Game/Blueprints/Items/BP_EquipableMaster.BP_EquipableMaster_C|GetEquipableInfo _equipableref))) (.Socketname (Utilities|Struct|BreakS_EquipableInfo (Variables|/Game/Blueprints/Items/BP_EquipableMaster.BP_EquipableMaster_C|GetEquipableInfo _equipableref)))))

(event Custom|MulticastWeaponEquip
  (params (Target :type Actor%20Object%20Reference) (SocketName :type Name) (EquippedState :type E_EquipableState%20Enum :default "NewEnumerator5"))
  ;[1 1 1] EquipWeapon
  (Utilities|IsValid Target
    (:Is%20Valid
      (bind _mesh (Variables|Character|GetMesh)
        (:then
          (Transformation|AttachComponentToComponent Target _mesh SocketName "KeepRelative" "KeepRelative" "KeepRelative" true)
          (Variables|Default|SetEquipState EquippedState))
        (:else)))))

(event Custom|SpawnEquipable_FP
  (params (Class :type Actor%20Class%20Reference) (SocketName :type Name))
  ;[1 1 1] EquipWeapon
  (bind _returnvalue (Game|SpawnActorfromClass Class (Math|Transform|MakeTransform "0, 0, 0" "0, 0, 0" "1.000000,1.000000,1.000000") "Undefined" 0 0))
  (bind _output_get (Variables|Default|SetFP_EquippedItem _returnvalue))
  (Actor|SetOwner _output_get self)
  (Transformation|AttachComponentToComponent _output_get (Variables|Default|GetFirstPersonMesh) SocketName "KeepRelative" "KeepRelative" "KeepRelative" true))

(event Custom|UnequipWeapon_TP
  ;[1 1 1] UnequipWeapon
  (Variables|Default|SetEquipState "NewEnumerator5"))

(event Custom|UnequipWeapon_FP
  ;[1 1 1] UnequipWeapon
  (Actor|DestroyActor (Variables|Default|GetFP_EquippedItem)))

(event Custom|AttackOnServer
  (bind _tp_equippeditem (Variables|Default|GetTP_EquippedItem)
    (:then
      (Class|BPIEquipableItem|UseItem(Message) _tp_equippeditem self))
    (:else)))

(event Custom|MontageMulticast
  (params (TP_Montage :type Anim%20Montage%20Object%20Reference))
  ;[1 1 1] MontagePlay
  (Animation|Montage|PlayMontage (Variables|Character|GetMesh) TP_Montage
    (:OnCompleted
      (bind _tp_equippeditem (Variables|Default|GetTP_EquippedItem)
        (:then
          (Class|BPIEquipableItem|EndAnimation(Message) _tp_equippeditem))
        (:else
          (Variables|Default|SetIsHarvesting false))))
    (:OnNotifyBegin
      (bind _tp_equippeditem_2 (Variables|Default|GetTP_EquippedItem)
        (:then
          (Class|BPIEquipableItem|Notify(Message) _tp_equippeditem_2))
        (:else)))))

(event Custom|MontageOnClient
  (params (FP_Montage :type Anim%20Montage%20Object%20Reference))
  ;[1 1 1] MontagePlay
  (Animation|Montage|PlayMontage (Variables|Default|GetFirstPersonMesh) FP_Montage))

(event Input|EnhancedActionEvents|EnhancedInputActionIA_OpenInviteList
  (params (ActionValue :type Boolean) (ElapsedSeconds :type Float%20%28double-precision%29) (TriggeredSeconds :type Float%20%28double-precision%29) (InputAction :type Input%20Action%20Object%20Reference :default "/Game/Input/Actions/IA_OpenInviteList.IA_OpenInviteList"))
  (:Started
    (bind _asbp_main_hud (Utilities|Casting|CastToBP_MainHUD (HUD|GetHUD (Game|GetPlayerController 0))))
    (Default|OpenInviteList _asbp_main_hud)))

(event Input|EnhancedActionEvents|EnhancedInputActionIA_Interact
  (params (ActionValue :type Boolean) (ElapsedSeconds :type Float%20%28double-precision%29) (TriggeredSeconds :type Float%20%28double-precision%29) (InputAction :type Input%20Action%20Object%20Reference :default "/Game/Input/Actions/IA_Interact.IA_Interact"))
  ;[1 1 1] Interact
  (:Started
    (CallFunction|InteractonServer)))

(event Input|EnhancedActionEvents|EnhancedInputActionIA_Attack
  (params (ActionValue :type Boolean) (ElapsedSeconds :type Float%20%28double-precision%29) (TriggeredSeconds :type Float%20%28double-precision%29) (InputAction :type Input%20Action%20Object%20Reference :default "/Game/Input/Actions/IA_Attack.IA_Attack"))
  (:Started
    (CallFunction|AttackonServer)))

(event EventBeginPlay)

(event Collision|EventActorBeginOverlap
  (params (OtherActor :type Actor%20Object%20Reference)))

(event EventTick
  (params (DeltaSeconds :type Float%20%28single-precision%29)))

(event EventFPMontage
  (params (FP_Montage :type Anim%20Montage%20Object%20Reference))
  ;[1 1 1] MontagePlay
  (CallFunction|MontageonClient FP_Montage))

(event EventTPMontage
  (params (TP_Montage :type Anim%20Montage%20Object%20Reference))
  ;[1 1 1] MontagePlay
  (CallFunction|MontageMulticast TP_Montage))

(event Input|KeyboardEvents|DebugKeyU
  (params (Key :type Key%20Structure :default "None") (ActionValue :type Input%20Action%20Value%20Structure))
  (:Pressed
    (bind _returnvalue (Utilities|GetDataTableRow "/Game/Blueprints/DataTables/DT_Items.DT_Items" "StoneHatchet")
      (:then
        (Default|AddItemonServer (Variables|Components|GetPlayerInventoryComponent) _returnvalue)))))

(event Input|KeyboardEvents|DebugKeyY
  (params (Key :type Key%20Structure :default "None") (ActionValue :type Input%20Action%20Value%20Structure))
  (:Pressed
    (bind _returnvalue (Utilities|GetDataTableRow "/Game/Blueprints/DataTables/DT_Items.DT_Items" "StonePickaxe")
      (:then
        (Default|AddItemonServer (Variables|Components|GetPlayerInventoryComponent) _returnvalue)))))

(event Input|KeyboardEvents|1
  (params (Key :type Key%20Structure :default "None"))
  ;[1 1 1] Hotbar binding
  (:Pressed
    (CallFunction|HotbaronServer)))

(event Input|KeyboardEvents|2
  (params (Key :type Key%20Structure :default "None"))
  ;[1 1 1] Hotbar binding
  (:Pressed
    (CallFunction|HotbaronServer 1)))

(event Input|KeyboardEvents|3
  (params (Key :type Key%20Structure :default "None"))
  ;[1 1 1] Hotbar binding
  (:Pressed
    (CallFunction|HotbaronServer 2)))

(event Input|KeyboardEvents|4
  (params (Key :type Key%20Structure :default "None"))
  ;[1 1 1] Hotbar binding
  (:Pressed
    (CallFunction|HotbaronServer 3)))

(event Input|KeyboardEvents|5
  (params (Key :type Key%20Structure :default "None"))
  ;[1 1 1] Hotbar binding
  (:Pressed
    (CallFunction|HotbaronServer 4)))

(event Input|KeyboardEvents|6
  (params (Key :type Key%20Structure :default "None"))
  ;[1 1 1] Hotbar binding
  (:Pressed
    (CallFunction|HotbaronServer 5)))

(event Input|KeyboardEvents|7
  (params (Key :type Key%20Structure :default "None"))
  ;[1 1 1] Hotbar binding
  (:Pressed
    (CallFunction|HotbaronServer 6)))

(event Input|KeyboardEvents|8
  (params (Key :type Key%20Structure :default "None"))
  ;[1 1 1] Hotbar binding
  (:Pressed
    (CallFunction|HotbaronServer 7)))

(fn ConstructionScript)

(fn UseHotbar
  (params (Index :type Integer))
  (bind _output_get (Variables|Default|SetHotbarIndex Index))
  (bind (_hasiteminslot_ _itemtype) (Default|CheckHotbar (Variables|Components|GetHotbarComponent) _output_get))
  (if _hasiteminslot_
    (switch Utilities|FlowControl|Switch|SwitchonE_ItemType _itemtype
      (:NewEnumerator1
        (Variables|Default|GetTP_EquippedItem
          (:then
            (Actor|DestroyActor (Variables|Default|GetTP_EquippedItem))
            (CallFunction|UnequipWeaponTP)
            (CallFunction|UnequipWeaponFP))
          (:else
            (CallFunction|SpawnEquipableTP (.ItemClass (Utilities|Struct|BreakS_ItemInfo (Utilities|Array|Get(acopy) (Variables|/Game/Blueprints/InventorySystem/Inventory/BP_ItemsContainerComponent.BP_ItemsContainerComponent_C|GetItems (Variables|Components|GetHotbarComponent)) (Variables|Default|GetHotbarIndex)))) (Utilities|Array|Get(acopy) (Variables|/Game/Blueprints/InventorySystem/Inventory/BP_ItemsContainerComponent.BP_ItemsContainerComponent_C|GetItems (Variables|Components|GetHotbarComponent)) (Variables|Default|GetHotbarIndex)) (Variables|Default|GetHotbarIndex))))))))

(fn HarvestLargeItem
  (params (Resource :type S%20Resource%20Structure%20Structure))
  (bind (_resourcename _quantity) (Utilities|Struct|BreakS_ResourceStructure Resource))
  (bind _returnvalue (Utilities|GetDataTableRow "/Game/Blueprints/DataTables/DT_Items.DT_Items" _resourcename)
    (:then
      (LocalVariables|SetLocalQuantity _quantity)
      (bind _output_get (LocalVariables|SetLocalOutRow _returnvalue))
      (bind _structout (Utilities|Struct|SetmembersinS_ItemInfo _output_get (LocalVariables|GetLocalQuantity)))
      (Default|AddItemonServer (Variables|Components|GetPlayerInventoryComponent) _structout)
      (bind _controllerref (Class|BPIController|GetControllerRef(Message) (Pawn|GetController)))
      (Default|ShowItemWidget _controllerref (.ItemIcon (Utilities|Struct|BreakS_ItemInfo (LocalVariables|GetLocalOutRow))) (LocalVariables|GetLocalQuantity) (.ItemName (Utilities|Struct|BreakS_ItemInfo (LocalVariables|GetLocalOutRow)))))))

(fn HarvestGroundItem
  (params (Ref :type Actor%20Object%20Reference))
  (bind _grounditemref (Class|BPIGroundItem|GetGroundItemRef(Message) Ref))
  (bind _output_get (LocalVariables|SetLocalHealth (- (Variables|/Game/Blueprints/HarvestingSystem/BP_GroundItemMaster.BP_GroundItemMaster_C|GetHealth _grounditemref) 15.0)))
  (if (<= _output_get 0.0)
    (bind _returnvalue (Utilities|GetDataTableRow "/Game/Blueprints/DataTables/DT_GroundResources.DT_GroundResources" (Utilities|String|StringToName (Utilities|GetClassDisplayName (Utilities|GetClass _grounditemref))))
      (:then
        (LocalVariables|SetLocalDestr (.Class (Utilities|Struct|BreakS_LargeItem _returnvalue)))
        (Utilities|IsValid _grounditemref
          (:Is%20Valid
            (LocalVariables|SetLocalTransform (Transformation|GetActorTransform _grounditemref))
            (Actor|DestroyActor _grounditemref)
            (Game|SpawnActorfromClass (LocalVariables|GetLocalDestr) (LocalVariables|GetLocalTransform) "Undefined" 0 "0.000000,0.000000,0.000000" 0)))))
    (else
      (Variables|/Game/Blueprints/HarvestingSystem/BP_GroundItemMaster.BP_GroundItemMaster_C|SetHealth _grounditemref (LocalVariables|GetLocalHealth))
      (bind _returnvalue_2 (Utilities|GetDataTableRow "/Game/Blueprints/DataTables/DT_GroundResources.DT_GroundResources" (Utilities|String|StringToName (Utilities|GetClassDisplayName (Utilities|GetClass _grounditemref))))
        (:then
          (bind _output_get_2 (LocalVariables|SetGivenResources (.GivenItems (Utilities|Struct|BreakS_LargeItem _returnvalue_2))))
          (for _array_element _output_get_2
            (bind _output_get_3 (LocalVariables|SetLocalQuan (Math|Float|Truncate (|((BaseVar*RateVar)*RandomVar) (Math|Conversions|ToFloat(Integer) (.Quantity (Utilities|Struct|BreakS_ResourceStructure _array_element))) 1.0 (Math|Random|RandomFloatinRange 0.3 1.2)))))
            (if (not (<= _output_get_3 0))
              (CallFunction|HarvestItemonServer (Utilities|Struct|MakeS_ResourceStructure (.ResourceName (Utilities|Struct|BreakS_ResourceStructure _array_element)) _output_get_3 "NewEnumerator0")))))))))

(fn CanCraftItem
  (params (Name :type Text) (Container :type E_ContainerType%20Enum :default "NewEnumerator0") (TableType :type E_CraftingType%20Enum :default "NewEnumerator0"))
  (bind _returnvalue (Utilities|GetDataTableRow (Utilities|Select :Index TableType :NewEnumerator0 "/Game/Blueprints/DataTables/DT_PlayerItemRecipes.DT_PlayerItemRecipes" :NewEnumerator1 0 :NewEnumerator2 0 :NewEnumerator3 0 :NewEnumerator4 0 :NewEnumerator5 0) (Utilities|String|StringToName (Utilities|String|ToString(Text) Name)))
    (:then
      (bind _cancraft_ (Default|ContainsItems (Utilities|Select :Index Container :NewEnumerator0 (Variables|Components|GetPlayerInventoryComponent) :NewEnumerator1 0 :NewEnumerator2 0 :NewEnumerator3 0) (Utilities|Struct|BreakS_ItemRecipe _returnvalue)))
      (return _cancraft_))))

(fn CraftItem
  (params (ItemName :type Text) (Container :type E_ContainerType%20Enum :default "NewEnumerator0") (TableType :type E_CraftingType%20Enum :default "NewEnumerator0"))
  (LocalVariables|SetLocalContainer Container)
  (bind _returnvalue (Utilities|GetDataTableRow (Utilities|Select :Index TableType :NewEnumerator0 "/Game/Blueprints/DataTables/DT_PlayerItemRecipes.DT_PlayerItemRecipes" :NewEnumerator1 0 :NewEnumerator2 0 :NewEnumerator3 0 :NewEnumerator4 0 :NewEnumerator5 0) (Utilities|String|StringToName (Utilities|String|ToString(Text) ItemName)))
    (:then
      (LocalVariables|SetLocalRequired (.RequiredItems (Utilities|Struct|BreakS_ItemRecipe _returnvalue)))
      (bind _cancraft_ (Default|ContainsItems (Utilities|Select :Index (LocalVariables|GetLocalContainer) :NewEnumerator0 (Variables|Components|GetPlayerInventoryComponent) :NewEnumerator1 0 :NewEnumerator2 0 :NewEnumerator3 0) (LocalVariables|GetLocalRequired)))
      (if _cancraft_
        (Default|RemoveItems (Utilities|Select :Index (LocalVariables|GetLocalContainer) :NewEnumerator0 (Variables|Components|GetPlayerInventoryComponent) :NewEnumerator1 0 :NewEnumerator2 0 :NewEnumerator3 0) (LocalVariables|GetLocalRequired))
        (bind _controllerref (Class|BPIController|GetControllerRef(Message) (Pawn|GetController)))
        (Default|ShowCraftingProgressBar _controllerref)
        (return true (Utilities|String|StringToName (Utilities|String|ToString(Text) (.ItemID (Utilities|Struct|BreakS_ItemRecipe _returnvalue)))) (LocalVariables|GetLocalContainer))
        (else
          (Development|PrintString "Cant  craft item")
          (return false "None" "NewEnumerator0"))))))

(fn AddCraftedItem
  (params (ItemNameToAdd :type Name) (Container] :type E_ContainerType%20Enum :default "NewEnumerator0"))
  (bind _returnvalue (Utilities|GetDataTableRow "/Game/Blueprints/DataTables/DT_Items.DT_Items" ItemNameToAdd)
    (:then
      (bind _output_get (LocalVariables|SetLocalOutRow _returnvalue))
      (bind _structout (Utilities|Struct|SetmembersinS_ItemInfo _output_get 1))
      (Default|AddItemonServer (Utilities|Select :Index Container] :NewEnumerator0 (Variables|Components|GetPlayerInventoryComponent) :NewEnumerator1 0 :NewEnumerator2 0 :NewEnumerator3 0) _structout))))

(fn GetArrowLocation
  (bind _arrow1 (Variables|Components|GetArrow1))
  (return (Transformation|GetWorldLocation _arrow1) (Transformation|GetWorldRotation _arrow1)))

(fn GetCharacterRef
  (return self))

(fn GetControllerfromChar
  (bind _controllerref (Class|BPIController|GetControllerRef(Message) (Pawn|GetController)))
  (return _controllerref))