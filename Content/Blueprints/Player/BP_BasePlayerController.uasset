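; Base player controller that owns the in-game HUD and relays inventory, hotbar and crafting updates to it.
; On BeginPlay, only the non-authority side creates and displays the main widget, which the open-inventory input toggles.
; Slot update and reset events find their widget by container type and index; storage and armor containers are not mapped.
; Other events forward item pickup notices, craft status and the crafting progress bar.
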(event Custom|InventoryOnClient
  (Default|ToggleInventory (Variables|Default|GetMainWidgetRef)))

(event Custom|ResetItemSlot
  (params (Container :type E_ContainerType%20Enum :default "NewEnumerator0") (Index :type Integer))
  (bind _slotwidget (CallFunction|GetInventoryWidget Container Index))
  (Utilities|IsValid _slotwidget
    (:Is%20Valid
      (Default|ResetSlot _slotwidget))))

(event Custom|UpdateItemSlot
  (params (Container :type E_ContainerType%20Enum :default "NewEnumerator0") (Index :type Integer) (ItemInfo :type S%20Item%20Info%20Structure))
  (bind _slotwidget (CallFunction|GetInventoryWidget Container Index))
  (Utilities|IsValid _slotwidget
    (:Is%20Valid
      (Default|UpdateSlot _slotwidget ItemInfo))))

(event Custom|ShowItemWidget
  (params (ResourceImage :type Texture%202D%20Object%20Reference) (ResourceQuantity :type Integer) (ResourceName :type Text))
  (Default|ShowItemCollected (Variables|Default|GetMainWidgetRef) ResourceImage ResourceQuantity ResourceName))

(event Custom|UpdateCraftStatus
  (params (bCanCraft :type Boolean))
  (Default|UpdateCraftStatus (Variables|/Game/UI/Inventory/WBP_Inventory.WBP_Inventory_C|GetCraftingWindow (Variables|/Game/UI/WBP_InGameMain.WBP_InGameMain_C|GetWBP_Inventory (Variables|Default|GetMainWidgetRef))) bCanCraft))

(event Custom|ShowCraftingProgressBar
  (Default|ShowCraftingBar (Variables|Default|GetMainWidgetRef)))

(event Input|EnhancedActionEvents|EnhancedInputActionIA_OpenInventory
  (params (ActionValue :type Boolean) (ElapsedSeconds :type Float%20%28double-precision%29) (TriggeredSeconds :type Float%20%28double-precision%29) (InputAction :type Input%20Action%20Object%20Reference :default "/Game/Input/Actions/IA_OpenInventory.IA_OpenInventory"))
  (:Started
    (CallFunction|InventoryonClient)))

(event EventBeginPlay
  (Networking|SwitchHasAuthority
    (:Remote
      (bind _returnvalue (UserInterface|CreateWidget "/Game/UI/WBP_InGameMain.WBP_InGameMain_C" (Game|GetPlayerController 0)))
      (bind _output_get (Variables|Default|SetMainWidgetRef _returnvalue))
      (UserInterface|Viewport|AddtoViewport _output_get 0))))

(fn ConstructionScript)

(fn GetInventoryWidget
  (params (Container :type E_ContainerType%20Enum :default "NewEnumerator0") (SlotIndex :type Integer))
  (return (Utilities|Array|Get(acopy) (Variables|/Game/UI/Inventory/WBP_ItemContainerGrid.WBP_ItemContainerGrid_C|GetSlots (Utilities|Select :Index Container :NewEnumerator0 (Variables|/Game/UI/Inventory/WBP_Inventory.WBP_Inventory_C|GetInventoryGrid (Variables|/Game/UI/WBP_InGameMain.WBP_InGameMain_C|GetWBP_Inventory (Variables|Default|GetMainWidgetRef))) :NewEnumerator1 (Variables|/Game/UI/Inventory/WBP_Hotbar.WBP_Hotbar_C|GetWBP_ItemContainerGrid (Variables|/Game/UI/WBP_InGameMain.WBP_InGameMain_C|GetWBP_Hotbar (Variables|Default|GetMainWidgetRef))) :NewEnumerator2 0 :NewEnumerator3 0)) SlotIndex)))

(fn GetControllerRef
  (return self))