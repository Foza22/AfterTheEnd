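; Player preview actor that films a stand-in character showing equipped items and armor, using a scene capture.
; On initialization it renders into a runtime render target, wraps it in a dynamic material and passes that to the player controller.
; Equip events spawn items onto mesh sockets and set an animation state, or fill four armor slots with pieces that follow the body mesh via leader pose.
; Unequip events destroy those actors.
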(event Custom|InitializeWindow
  (params (PlayerControllerRef :type BP%20Base%20Player%20Controller%20Object%20Reference))
  (bind _returnvalue (Rendering|CreateRenderTarget2D 500 800 "RTF_RGBA16f"))
  (Variables|/Script/Engine.SceneCaptureComponent2D|SetTextureTarget (Variables|Default|GetSceneCaptureComponent2D) _returnvalue)
  (bind _returnvalue_2 (Rendering|Material|CreateDynamicMaterialInstance "/Game/Blueprints/Player/PlayerWindow/M_PlayerWindow.M_PlayerWindow" "None" "None" :!class /Script/Engine.KismetMaterialLibrary))
  (Rendering|Material|SetTextureParameterValue _returnvalue_2 "Param" _returnvalue)
  (Utilities|IsValid PlayerControllerRef
    (:Is%20Valid
      (Default|SetRenderMaterial PlayerControllerRef _returnvalue_2))))

(event Custom|EquipItem
  (params (Info :type S%20Equipable%20Info%20Structure))
  (bind (_socketname _animationstate _firstpersonequipclass) (Utilities|Struct|BreakS_EquipableInfo Info))
  (Variables|Default|SetEquippedState _animationstate)
  (bind _returnvalue (Game|SpawnActorfromClass _firstpersonequipclass (Math|Transform|MakeTransform "0, 0, 0" "0, 0, 0" "1.000000,1.000000,1.000000") "Undefined" 0 0))
  (bind _asbp_fp_base_hatchet (Utilities|Casting|CastToBP_FP_BaseHatchet _returnvalue))
  (Rendering|SetOnlyOwnerSee (Variables|/Game/Blueprints/Items/Equipables/Tools/BP_FP_BaseHatchet.BP_FP_BaseHatchet_C|GetStaticMesh _asbp_fp_base_hatchet) false :!class /Script/Engine.PrimitiveComponent)
  (bind _output_get (Variables|Default|SetEquippedItem _returnvalue))
  (Transformation|AttachComponentToComponent _output_get (Variables|Default|GetSkeletalMesh) _socketname "SnapToTarget" "SnapToTarget" "KeepRelative" true))

(event Custom|UnequipItem
  (bind _equippeditem (Variables|Default|GetEquippedItem)
    (:then
      (Actor|DestroyActor _equippeditem)
      (Variables|Default|SetEquippedState "NewEnumerator5"))
    (:else)))

(event Custom|EquipArmor
  (params (ItemInfo :type S%20Item%20Info%20Structure))
  (CallFunction|EquipArmorFunc ItemInfo))

(event Custom|UnequipArmor
  (params (ArmorType :type E_ArmorType%20Enum :default "NewEnumerator0"))
  (switch Utilities|FlowControl|Switch|SwitchonE_ArmorType ArmorType
    (:NewEnumerator0
      (bind _helmetslot (Variables|Default|GetHelmetSlot)
        (:then
          (Actor|DestroyActor _helmetslot))
        (:else)))
    (:NewEnumerator1
      (bind _chestslot (Variables|Default|GetChestSlot)
        (:then
          (Actor|DestroyActor _chestslot))
        (:else)))
    (:NewEnumerator2
      (bind _pantsslot (Variables|Default|GetPantsSlot)
        (:then
          (Actor|DestroyActor _pantsslot))
        (:else)))
    (:NewEnumerator3
      (bind _bootsslot (Variables|Default|GetBootsSlot)
        (:then
          (Actor|DestroyActor _bootsslot))
        (:else)))))

(fn ConstructionScript)

(fn EquipArmorFunc
  (params (ItemInfo :type S%20Item%20Info%20Structure))
  (bind (_itemclass _armortype) (Utilities|Struct|BreakS_ItemInfo ItemInfo))
  (LocalVariables|SetLocalArmor _armortype)
  (bind _returnvalue (Game|SpawnActorfromClass _itemclass (Math|Transform|MakeTransform "0, 0, 0" "0, 0, 0" "1.000000,1.000000,1.000000") "Undefined" 0 0))
  (switch Utilities|FlowControl|Switch|SwitchonE_ArmorType (LocalVariables|GetLocalArmor)
    (:NewEnumerator0
      (bind _output_get (Variables|Default|SetHelmetSlot _returnvalue)))
    (:NewEnumerator1
      (bind _output_get_2 (Variables|Default|SetChestSlot _returnvalue)))
    (:NewEnumerator2
      (bind _output_get_3 (Variables|Default|SetPantsSlot _returnvalue)))
    (:NewEnumerator3
      (bind _output_get_4 (Variables|Default|SetBootsSlot _returnvalue))))
  (Transformation|AttachComponentToComponent (Utilities|Select :Index (LocalVariables|GetLocalArmor) :NewEnumerator0 _output_get :NewEnumerator1 _output_get_2 :NewEnumerator2 _output_get_3 :NewEnumerator3 _output_get_4) (Variables|Default|GetSkeletalMesh) "None" "SnapToTarget" "SnapToTarget" "SnapToTarget" true)
  (bind _armorref (Class|BPIArmorItem|GetArmorRef(Message) (Utilities|Select :Index (LocalVariables|GetLocalArmor) :NewEnumerator0 _output_get :NewEnumerator1 _output_get_2 :NewEnumerator2 _output_get_3 :NewEnumerator3 _output_get_4)))
  (Components|SkinnedMesh|SetLeaderPoseComponent (Variables|/Game/Blueprints/Items/BP_ArmorMaster.BP_ArmorMaster_C|GetSkeletalMesh _armorref) (Variables|Default|GetSkeletalMesh) false false))

(fn GetPlayerWindowRef
  (return self))