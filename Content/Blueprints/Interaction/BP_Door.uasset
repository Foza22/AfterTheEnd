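; Interactable door Blueprint that toggles between open and closed when used.
; On BeginPlay it binds to the Interaction component's OnInteract event, which checks IsClosed to call OpenDoor or CloseDoor.
; Each snaps the Door component's relative rotation with no animation and updates the flag.
; An unrelated DetectOptimalGraphics function, not called here, runs a hardware benchmark and applies the resulting graphics settings.
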(event Custom|OnInteract_Event
  (params (Instigator :type Actor%20Object%20Reference))
  (if (Variables|Default|GetIsClosed)
    (CallFunction|OpenDoor)
    (else
      (CallFunction|CloseDoor))))

(event Custom|OpenDoor
  (Transformation|SetRelativeRotation (Variables|Default|GetDoor) "0.000000,90.000000,0.000000" false false)
  (Variables|Default|SetIsClosed false))

(event Custom|CloseDoor
  (Transformation|SetRelativeRotation (Variables|Default|GetDoor) "0, 0, 0" false false)
  (Variables|Default|SetIsClosed true))

(event EventBeginPlay
  (EventDispatchers|AssignOnInteract (Variables|Default|GetInteraction) (delegate Custom|OnInteract_Event)))

(event Collision|EventActorBeginOverlap
  (params (OtherActor :type Actor%20Object%20Reference)))

(event EventTick
  (params (DeltaSeconds :type Float%20%28single-precision%29)))

(fn ConstructionScript
  (|CallParentFunction))

(fn DetectOptimalGraphics
  (bind _returnvalue (Settings|GetGameUserSettings))
  (Class|GameUserSettings|RunHardwareBenchmark _returnvalue 10 1.0 1.0)
  (Class|GameUserSettings|ApplyHardwareBenchmarkResults _returnvalue))