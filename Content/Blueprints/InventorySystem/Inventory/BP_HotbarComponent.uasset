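; Inventory component for the player's hotbar, extending a base container component with slot and equipment hooks.
; Dropped slots from the player inventory or hotbar are moved in through TransferItem, and CheckHotbar reports whether a slot holds an item and its type.
; Add and remove overrides call the parent, then update or reset the slot through the owner's controller; removal also tells the character to unequip that index.
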(event EventBeginPlay
  (|CallParentFunction) ; This node is disabled and will not be called.\nDrag off pins to build functionality.
)

(event EventTick
  (params (DeltaSeconds :type Float%20%28single-precision%29))
  (|CallParentFunction DeltaSeconds) ; This node is disabled and will not be called.\nDrag off pins to build functionality.
)

(fn CheckHotbar
  (params (Index :type Integer))
  (bind _items (Variables|Default|GetItems))
  (bind _output (Utilities|Array|Get(acopy) _items Index))
  (bind (_itemid _itemquantity _itemicon _itemname _itemdesc _itemdamage _itemrarity _itemcurhp _itemmaxhp _isstackable_ _stacksize _itemtype) (Utilities|Struct|BreakS_ItemInfo _output))
  (if (== _itemid 0)
    (return false "NewEnumerator0")
    (else
      (return true _itemtype))))

(fn HandleSlotDrop
  (params (From%20Container :type BP%20Items%20Container%20Component%20Object%20Reference) (From%20Index :type Integer) (ToIndex :type Integer))
  (LocalVariables|SetLocalFromContainer From%20Container)
  (LocalVariables|SetLocalFromIndex From%20Index)
  (LocalVariables|SetLocalToIndex ToIndex)
  (switch Utilities|FlowControl|Switch|SwitchonE_ContainerType (Variables|/Game/Blueprints/InventorySystem/Inventory/BP_ItemsContainerComponent.BP_ItemsContainerComponent_C|GetContainerType (LocalVariables|GetLocalFromContainer))
    (:NewEnumerator0
      _)
    (:NewEnumerator1
      _))
  (Default|TransferItem (LocalVariables|GetLocalFromContainer) self (LocalVariables|GetLocalToIndex) (LocalVariables|GetLocalFromIndex))
  (return))

(fn AddItemtoIndex
  (params (Item :type S%20Item%20Info%20Structure) (ToIndex :type Integer) (FromIndex :type Integer))
  (bind _bsuccess (|CallParentFunction Item ToIndex FromIndex))
  (bind _controllerref (Class|BPICharacter|GetControllerfromChar(Message) (Components|GetOwner)))
  (Default|UpdateItemSlot _controllerref (Variables|Default|GetContainerType) ToIndex (CallFunction|GetItematIndex ToIndex))
  (return _bsuccess))

(fn RemoveItematIndex
  (params (Index :type Integer))
  (bind _bsuccess (|CallParentFunction Index))
  (bind _controllerref (Class|BPICharacter|GetControllerfromChar(Message) (Components|GetOwner)))
  (Default|ResetItemSlot _controllerref (Variables|Default|GetContainerType) Index)
  (bind _characterref (Class|BPICharacter|GetCharacterRef(Message) (Components|GetOwner)))
  (Default|UnequipCurrentItem _characterref Index)
  (return _bsuccess))