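; BP_WallMaster is a wall piece in the building system, named as the master Blueprint for walls.
; GetBoxes returns its seven box components: two each for ceilings, triangle ceilings and torches, plus one for a wall, apparently attachment points for other pieces.
; The construction script only calls the parent's, and the event graph holds no active logic.
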(event EventBeginPlay)

(event Collision|EventActorBeginOverlap
  (params (OtherActor :type Actor%20Object%20Reference)))

(event EventTick
  (params (DeltaSeconds :type Float%20%28single-precision%29)))

(fn ConstructionScript
  (|CallParentFunction))

(fn GetBoxes
  (return (Utilities|Array|MakeArray (Variables|Default|GetCeiling) (Variables|Default|GetCeiling1) (Variables|Default|GetTriangleCeiling) (Variables|Default|GetTriangleCeiling1) (Variables|Default|GetTorchBox) (Variables|Default|GetTorchBox1) (Variables|Default|GetWall))))