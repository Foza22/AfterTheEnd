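; BP_TriangleFoundationMaster is a triangle foundation Blueprint for the building system.
; Its GetBoxes function returns a fixed array of its components, named for the triangle foundation, foundation, wall and ramp pieces, likely attachment boxes for those types.
; The construction script only calls the parent, and the event graph holds no active logic.
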(event EventBeginPlay)

(event Collision|EventActorBeginOverlap
  (params (OtherActor :type Actor%20Object%20Reference)))

(event EventTick
  (params (DeltaSeconds :type Float%20%28single-precision%29)))

(fn ConstructionScript
  (|CallParentFunction))

(fn GetBoxes
  (return (Utilities|Array|MakeArray (Variables|Default|GetTriangleFoundation2) (Variables|Default|GetWall2) (Variables|Default|GetWall1) (Variables|Default|GetWall) (Variables|Default|GetFoundation) (Variables|Default|GetTriangleFoundation1) (Variables|Default|GetTriangleFoundation) (Variables|Default|GetFoundation1) (Variables|Default|GetFoundation2) (Variables|Default|GetRamp) (Variables|Default|GetRamp1))))