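; BP_BuildableMaster is the base building-system structure, handling damage and destruction.
; It subtracts damage only when the causer implements BPI_StructureDamage and lists this StructureTier among its damageable types.
; At zero HP, a multicast event swaps the static mesh for a physics-simulated destructible mesh and spawns FS_DestructionForce at its location.
; GetBuildableRef returns the actor itself, while GetBoxes is an empty stub.
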(event Custom|MulticastDestruction
  (bind _staticmesh (Variables|Default|GetStaticMesh))
  (bind _destructablemesh (Variables|Default|GetDestructableMesh))
  (Collision|SetCollisionEnabled _staticmesh "NoCollision")
  (Rendering|SetVisibility _staticmesh false false)
  (Rendering|SetVisibility _destructablemesh true false)
  (Physics|SetSimulatePhysics _destructablemesh true)
  (Development|SetHiddeninGame _destructablemesh false false)
  (Game|SpawnActorfromClass "/Game/Blueprints/HarvestingSystem/Destructables/FS_DestructionForce.FS_DestructionForce_C" (Math|Transform|MakeTransform (Transformation|GetActorLocation) "0, 0, 0" "1.000000,1.000000,1.000000") "Undefined" 0 0))

(event Game|Damage|EventAnyDamage
  (params (Damage :type Float%20%28single-precision%29) (DamageType :type Damage%20Type%20Object%20Reference) (InstigatedBy :type Controller%20Object%20Reference) (DamageCauser :type Actor%20Object%20Reference))
  (if (Utilities|DoesObjectImplementInterface DamageCauser "/Game/Blueprints/Interfaces/BPI_StructureDamage.BPI_StructureDamage_C")
    (bind _canapplydamage (CallFunction|CanDamageStructure DamageCauser))
    (if _canapplydamage
      (Variables|Default|SetCurrentHP (- (Variables|Default|GetCurrentHP) Damage))
      (if (<= (Variables|Default|GetCurrentHP) 0.0)
        (CallFunction|DestroyStructure)))))

(event EventDestroyStructure
  (CallFunction|MulticastDestruction))

(fn ConstructionScript)

(fn CanDamageStructure
  (params (Instigator :type Object%20Object%20Reference))
  (Utilities|IsValid Instigator
    (:Is%20Valid
      (bind _damagetiers (Class|BPIStructureDamage|GetCanDamage(Message) Instigator))
      (bind _array_element (Utilities|Array|ForEachLoopwithBreak (Utilities|Struct|BreakS_DamageTiers _damagetiers) :!label _label)
        (:LoopBody
          (if (Utilities|Enum|Equal(Enum) _array_element (Variables|Default|GetStructureTier))
            (LocalVariables|SetbCanDamage true)
            (goto _label Break)))
        (:Completed
          (return (LocalVariables|GetbCanDamage)))))))

(fn GetBoxes
  (return 0))

(fn GetBuildableRef
  (return self))