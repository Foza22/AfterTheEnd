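; Base door Blueprint for the building system that swings open and closed when interacted with.
; Interact toggles the replicated IsDoorOpen flag, and its OnRep passes the new state to SetDoorRotation.
; SetDoorRotation plays or reverses a Timeline that drives the static mesh's relative yaw, so the animation follows replicated state.
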(event Custom|SetDoorRotation
  (params (bOpenDoor :type Boolean))
  (if bOpenDoor
    (bind _newtrack_0 (Timeline|Timeline Play)
      (:Update
        (Transformation|SetRelativeRotation (Variables|Default|GetStaticMesh) (Math|Rotator|MakeRotator 0.0 0.0 _newtrack_0) false false)))
    (else
      (Timeline|Timeline Reverse))))

(event EventBeginPlay)

(event Collision|EventActorBeginOverlap
  (params (OtherActor :type Actor%20Object%20Reference)))

(event EventTick
  (params (DeltaSeconds :type Float%20%28single-precision%29)))

(event EventInteract
  (params (Instigator :type BP%20Base%20Character%20Object%20Reference))
  (if (Variables|Default|GetbIsDoorOpen?)
    (Variables|Default|SetbIsDoorOpen? false)
    (else
      (Variables|Default|SetbIsDoorOpen? true))))

(fn ConstructionScript
  (|CallParentFunction))

(fn OnRepBIsDoorOpen?
  (CallFunction|SetDoorRotation (Variables|Default|GetbIsDoorOpen?)))