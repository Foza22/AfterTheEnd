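; Base foundation piece for the building system, exposing the boxes that belong to it for other building logic to query.
; GetBoxes returns a fixed array of box components named for square foundations, triangle foundations, walls, ramps and stairs, apparently sockets for neighboring pieces.
; The event graph is empty and the construction script only calls its parent.
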(event EventBeginPlay)

(event Collision|EventActorBeginOverlap
  (params (OtherActor :type Actor%20Object%20Reference)))

(event EventTick
  (params (DeltaSeconds :type Float%20%28single-precision%29)))

(fn ConstructionScript
  (|CallParentFunction))

(fn GetBoxes
  (return (Utilities|Array|MakeArray (Variables|Default|GetFoundation) (Variables|Default|GetFoundation1) (Variables|Default|GetFoundation2) (Variables|Default|GetFoundation3) (Variables|Default|GetWall) (Variables|Default|GetWall1) (Variables|Default|GetWall2) (Variables|Default|GetWall3) (Variables|Default|GetTriangleFoundation) (Variables|Default|GetTriangleFoundation3) (Variables|Default|GetTriangleFoundation1) (Variables|Default|GetTriangleFoundation2) (Variables|Default|GetRamp) (Variables|Default|GetRamp1) (Variables|Default|GetRamp2) (Variables|Default|GetRamp3) (Variables|Default|GetStairsBox))))