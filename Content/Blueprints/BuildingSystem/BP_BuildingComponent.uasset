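; Building component that lets a player place structures from DT_Structures using a green or red preview.
; The client loops a camera line trace, snapping to the hit actor's box components and validating overlap, ground support and "Foundation"-tagged support.
; On the server, SpawnBuildOnServer repeats the checks from the sent camera vector and rotation, then spawns the structure at the client-supplied transform if they pass.
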(event Custom|LaunchBuildMode
  (params (StructureName :type Text))
  ;[1 1 1] Build Mode On Client
  (if (Variables|Default|GetIsBuildModeEnabled)
    (CallFunction|StopBuildLoop)
    (else
      (Variables|Default|SetIsBuildModeEnabled true)
      (CallFunction|BuildModeClient (Variables|Default|GetStructureDebug)))))

(event Custom|BuildLoop
  (bind _buildpreview (Variables|Default|GetBuildPreview))
  ;[1 1 1] Build Mode On Client
  (if (Variables|Default|GetIsBuildModeEnabled)
    (Utilities|FlowControl|Delay 0.01)
    (CallFunction|BuildModeClient)
    (else
      (Variables|Default|SetIsBuildModeEnabled false)
      (Utilities|IsValid _buildpreview
        (:Is%20Valid
          (Actor|DestroyActor _buildpreview))))))

(event Custom|StopBuildLoop
  (bind _buildpreview (Variables|Default|GetBuildPreview))
  ;[1 1 1] Build Mode On Client
  (Variables|Default|SetIsBuildModeEnabled false)
  (Utilities|IsValid _buildpreview
    (:Is%20Valid
      (Actor|DestroyActor _buildpreview))))

(event Custom|SpawnBuildOnServer
  (params (Transform :type Transform) (StructureName :type Text) (ClientCameraVector :type Vector) (ClientCameraRotation :type Rotator))
  (Networking|SwitchHasAuthority
    (:Authority
      (Variables|Default|SetBuildTransform Transform)
      (bind _bcanbuild (CallFunction|BuildPlacementCheck StructureName ClientCameraVector ClientCameraRotation))
      (if _bcanbuild
        (CallFunction|SpawnBuildable Transform StructureName)
        (else
          (bind _buildpreview (Variables|Default|GetBuildPreview)
            (:then
              _)
            (:else))))
      (Actor|DestroyActor _buildpreview))))

(fn BuildModeClient
  (params (StructureName :type Text))
  (bind _buildpreview (Variables|Default|GetBuildPreview))
  (bind _buildableinfo (Variables|/Game/Blueprints/BuildingSystem/BP_BuildableMaster.BP_BuildableMaster_C|GetBuildableInfo _buildpreview))
  (bind (_canplaceonground _canplaceonfoundation) (Utilities|Struct|BreakS_BuildableInfo _buildableinfo))
  (bind _characterref (Class|BPICharacter|GetCharacterRef(Message) (Components|GetOwner)))
  (Variables|Default|GetBuildPreview
    (:then
      _)
    (:else
      (CallFunction|SpawnBuildPreview StructureName)
      (bind _buildpreview_2 (Variables|Default|GetBuildPreview)
        (:then
          _)
        (:else))))
  (bind (_outhit _returnvalue) (Collision|LineTraceByChannel (+ (Transformation|GetWorldLocation (Variables|/Script/AfterTheEnd.BaseCharacter|GetFirstPersonCamera _characterref)) (* (Math|Vector|GetForwardVector (Variables|/Script/AfterTheEnd.BaseCharacter|GetFirstPersonCamera _characterref)) (LocalVariables|GetBuildDistanceClose))) (+ (Transformation|GetWorldLocation (Variables|/Script/AfterTheEnd.BaseCharacter|GetFirstPersonCamera _characterref)) (* (Math|Vector|GetForwardVector (Variables|/Script/AfterTheEnd.BaseCharacter|GetFirstPersonCamera _characterref)) (LocalVariables|GetBuildDistanceFar))) (Utilities|Struct|BreakS_BuildableInfo (Variables|/Game/Blueprints/BuildingSystem/BP_BuildableMaster.BP_BuildableMaster_C|GetBuildableInfo _buildpreview_2)) false (Utilities|Array|MakeArray _buildpreview_2) "None"))
  (if _returnvalue
    (Variables|Default|SetHitActor (.HitActor (Collision|BreakHitResult _outhit)))
    (Variables|Components|SetHitComponent (.HitComponent (Collision|BreakHitResult _outhit)))
    (bind _characterref_2 (Class|BPICharacter|GetCharacterRef(Message) (Components|GetOwner)))
    (Variables|Default|SetBuildTransform (Math|Transform|MakeTransform (.ImpactPoint (Collision|BreakHitResult _outhit)) (Math|Rotator|MakeRotator 0.0 0.0 (+ (.yaw (Transformation|GetWorldRotation (Variables|/Script/AfterTheEnd.BaseCharacter|GetFirstPersonCamera _characterref_2))) 9e+01)) "1.000000,1.000000,1.000000"))
    (Utilities|IsValid (Variables|Default|GetBuildPreview)
      (:Is%20Valid
        (bind (_bfound _location) (CallFunction|GetSnappingPoints))
        (if _bfound
          (Variables|Default|SetBuildTransform _location)
          (if (Utilities|Struct|BreakS_BuildableInfo (Variables|/Game/Blueprints/BuildingSystem/BP_BuildableMaster.BP_BuildableMaster_C|GetBuildableInfo (Variables|Default|GetBuildPreview)))
            (bind _bdidhit (CallFunction|IsBuildFloating :!label _label))
            (bind _boverlapping (CallFunction|CheckforOverlap))
            (if (and (not _boverlapping) _bdidhit)
              (CallFunction|SetPreviewColor true)
              (CallFunction|BuildLoop)
              (else
                (if _canplaceonfoundation :!label _label_2
                  (bind _bonfoundation (CallFunction|IsBuildonFoundation))
                  (bind _boverlapping_2 (CallFunction|CheckforOverlap))
                  (CallFunction|SetPreviewColor (and (not _boverlapping_2) _bonfoundation))
                  (CallFunction|BuildLoop)
                  (else
                    (CallFunction|SetPreviewColor false)
                    (CallFunction|BuildLoop)))))
            (else
              (bind _boverlapping_3 (CallFunction|CheckforOverlap))
              (CallFunction|SetPreviewColor (not _boverlapping_3))
              (CallFunction|BuildLoop)))
          (elif _canplaceonground
            (goto _label)
            (else
              (goto _label_2)))))
      (:Is%20Not%20Valid
        (CallFunction|SpawnBuildPreview)
        (CallFunction|BuildLoop)))
    (else
      (bind _characterref_3 (Class|BPICharacter|GetCharacterRef(Message) (Components|GetOwner)))
      (Variables|Default|SetBuildTransform (Math|Transform|MakeTransform (.TraceEnd (Collision|BreakHitResult _outhit)) (Math|Rotator|MakeRotator 0.0 0.0 (+ (.yaw (Transformation|GetWorldRotation (Variables|/Script/AfterTheEnd.BaseCharacter|GetFirstPersonCamera _characterref_3))) 9e+01)) "1.000000,1.000000,1.000000"))
      (Utilities|IsValid (Variables|Default|GetBuildPreview)
        (:Is%20Valid
          (CallFunction|SetPreviewColor false)
          (CallFunction|BuildLoop))
        (:Is%20Not%20Valid
          (CallFunction|SpawnBuildPreview)
          (CallFunction|BuildLoop))))))

(fn SpawnBuildPreview
  (params (StructureName :type Text))
  (bind _returnvalue (Utilities|GetDataTableRow "/Game/Blueprints/BuildingSystem/Misc/DT_Structures.DT_Structures" (Utilities|String|StringToName (Utilities|String|ToString(Text) StructureName)))
    (:then
      (bind _returnvalue_2 (Game|SpawnActorfromClass (Utilities|Struct|BreakS_BuildTableInfo _returnvalue) (Variables|Default|GetBuildTransform) "Undefined" 0 0))
      (bind _output_get (Variables|Default|SetBuildPreview _returnvalue_2))
      (Collision|SetCollisionEnabled (Variables|/Game/Blueprints/BuildingSystem/BP_BuildableMaster.BP_BuildableMaster_C|GetStaticMesh _output_get) "NoCollision"))))

(fn SetPreviewColor
  (params (IsGreen :type Boolean))
  (LocalVariables|SetLocalCanPlace IsGreen)
  (for _array_element (Actor|GetComponentsByClass (Variables|Default|GetBuildPreview) "/Script/Engine.StaticMeshComponent")
    (for _index (range 0 (- (Rendering|Material|GetNumMaterials _array_element) 1))
      (if (LocalVariables|GetLocalCanPlace)
        (Rendering|Material|SetMaterial _array_element _index "/Game/Blueprints/BuildingSystem/Materials/MI_Green.MI_Green")
        (else
          (Rendering|Material|SetMaterial _array_element _index "/Game/Blueprints/BuildingSystem/Materials/MI_Red.MI_Red"))))
    (Transformation|SetWorldTransform (Variables|/Game/Blueprints/BuildingSystem/BP_BuildableMaster.BP_BuildableMaster_C|GetDefaultSceneRoot (Variables|Default|GetBuildPreview)) (Variables|Default|GetBuildTransform) false false)))

(fn SpawnBuildable
  (params (Transform :type Transform) (BuildName :type Text))
  (LocalVariables|SetLocalTransform Transform)
  (bind _returnvalue (Utilities|GetDataTableRow "/Game/Blueprints/BuildingSystem/Misc/DT_Structures.DT_Structures" (Utilities|String|StringToName (Utilities|String|ToString(Text) BuildName)))
    (:then
      (Game|SpawnActorfromClass (Utilities|Struct|BreakS_BuildTableInfo _returnvalue) (LocalVariables|GetLocalTransform) "Undefined" 0 0))))

(fn CheckforOverlap
  (bind _buildpreview (Variables|Default|GetBuildPreview))
  (bind _buildpreview_2 (Variables|Default|GetBuildPreview))
  (bind _buildpreview_3 (Variables|Default|GetBuildPreview))
  (bind _buildpreview_4 (Variables|Default|GetBuildPreview))
  (bind _buildableinfo (Variables|/Game/Blueprints/BuildingSystem/BP_BuildableMaster.BP_BuildableMaster_C|GetBuildableInfo _buildpreview))
  (bind _staticmesh (Variables|/Game/Blueprints/BuildingSystem/BP_BuildableMaster.BP_BuildableMaster_C|GetStaticMesh _buildpreview_2))
  (bind _overlapboxsize (Variables|/Game/Blueprints/BuildingSystem/BP_BuildableMaster.BP_BuildableMaster_C|GetOverlapBoxSize _buildpreview_3))
  (bind _rootcomponent (Variables|/Script/Engine.Actor|GetRootComponent _buildpreview_4))
  (bind (_origin _boxextent) (Collision|GetComponentBounds _staticmesh))
  (bind (_origin_2 _boxextent_2) (Collision|GetComponentBounds _overlapboxsize))
  (bind _returnvalue (Transformation|GetWorldRotation _rootcomponent))
  (bind _returnvalue_2 (select (.usecustomoverlap _buildableinfo) _origin_2 _origin))
  (bind _returnvalue_3 (Collision|BoxTraceByChannel _returnvalue_2 _returnvalue_2 (/ (select (.usecustomoverlap _buildableinfo) _boxextent_2 _boxextent) (LocalVariables|GetHalfSize)) (Math|Rotator|MakeRotator (.roll _returnvalue) (.pitch _returnvalue) (+ (.yaw _returnvalue) 9e+01)) "TraceTypeQuery1" false (Utilities|Array|MakeArray (Variables|Default|GetBuildPreview)) "None"))
  (return _returnvalue_3))

(fn BuildPlacementCheck
  (params (StructureName :type Text) (ClientCameraVector :type Vector) (ClientCameraRotation :type Rotator))
  (bind _buildpreview (Variables|Default|GetBuildPreview))
  (bind _buildableinfo (Variables|/Game/Blueprints/BuildingSystem/BP_BuildableMaster.BP_BuildableMaster_C|GetBuildableInfo _buildpreview))
  (bind (_canplaceonground _canplaceonfoundation) (Utilities|Struct|BreakS_BuildableInfo _buildableinfo))
  (bind _characterref (Class|BPICharacter|GetCharacterRef(Message) (Components|GetOwner)))
  (LocalVariables|SetLocalCameraRotation ClientCameraRotation)
  (CallFunction|SpawnBuildPreview StructureName)
  (bind _buildpreview_2 (Variables|Default|GetBuildPreview)
    (:then
      (bind (_outhit _returnvalue) (Collision|LineTraceByChannel (+ (Transformation|GetWorldLocation (Variables|/Script/AfterTheEnd.BaseCharacter|GetFirstPersonCamera _characterref)) (* ClientCameraVector (LocalVariables|GetBuildDistClose))) (+ (Transformation|GetWorldLocation (Variables|/Script/AfterTheEnd.BaseCharacter|GetFirstPersonCamera _characterref)) (* ClientCameraVector (LocalVariables|GetBuildDistFar))) (Utilities|Struct|BreakS_BuildableInfo (Variables|/Game/Blueprints/BuildingSystem/BP_BuildableMaster.BP_BuildableMaster_C|GetBuildableInfo _buildpreview_2)) false (Utilities|Array|MakeArray _buildpreview_2) "None"))
      (if _returnvalue
        (Variables|Default|SetHitActor (.HitActor (Collision|BreakHitResult _outhit)))
        (Variables|Components|SetHitComponent (.HitComponent (Collision|BreakHitResult _outhit)))
        (Variables|Default|SetBuildTransform (Math|Transform|MakeTransform (.ImpactPoint (Collision|BreakHitResult _outhit)) (Math|Rotator|MakeRotator (.roll (LocalVariables|GetLocalCameraRotation)) (.pitch (LocalVariables|GetLocalCameraRotation)) (+ (.yaw (LocalVariables|GetLocalCameraRotation)) 9e+02)) "1.000000,1.000000,1.000000"))
        (Utilities|IsValid (Variables|Default|GetBuildPreview)
          (:Is%20Valid
            (bind (_bfound _location) (CallFunction|GetSnappingPoints))
            (if _bfound
              (Variables|Default|SetBuildTransform _location)
              (if (Utilities|Struct|BreakS_BuildableInfo (Variables|/Game/Blueprints/BuildingSystem/BP_BuildableMaster.BP_BuildableMaster_C|GetBuildableInfo (Variables|Default|GetBuildPreview)))
                (bind _bdidhit (CallFunction|IsBuildFloating :!label _label))
                (bind _boverlapping (CallFunction|CheckforOverlap))
                (if (and (not _boverlapping) _bdidhit)
                  _
                  (else
                    (if _canplaceonfoundation :!label _label_2
                      (bind _boverlapping_2 (CallFunction|CheckforOverlap))
                      (bind _bonfoundation (CallFunction|IsBuildonFoundation))
                      (return (and (not _boverlapping_2) _bonfoundation))
                      (else
                        (return false)))))
                (else
                  (bind _boverlapping_3 (CallFunction|CheckforOverlap))
                  (return (not _boverlapping_3))))
              (elif _canplaceonground
                (goto _label)
                (else
                  (goto _label_2))))
            (return true))
          (:Is%20Not%20Valid
            _))
        (else
          (Variables|Default|SetBuildTransform (Math|Transform|MakeTransform (.TraceEnd (Collision|BreakHitResult _outhit)) (Math|Rotator|MakeRotator (.roll (LocalVariables|GetLocalCameraRotation)) (.pitch (LocalVariables|GetLocalCameraRotation)) (+ (.yaw (LocalVariables|GetLocalCameraRotation)) 9e+02)) "1.000000,1.000000,1.000000"))
          (Utilities|IsValid (Variables|Default|GetBuildPreview)
            (:Is%20Valid
              _)
            (:Is%20Not%20Valid
              _))))
      (return false))
    (:else)))

(fn GetSnappingPoints
  (bind _boxesref (Class|BPIBuildable|GetBoxes(Message) (Variables|Default|GetHitActor)))
  (bind _array_element (Utilities|Array|ForEachLoopwithBreak _boxesref :!label _label)
    (:LoopBody
      (bind _hitcomponent (Variables|Components|GetHitComponent)
        (:then
          (if (== _array_element _hitcomponent)
            (LocalVariables|SetbLocalFound true)
            (goto _label Break)))
        (:else)))
    (:Completed
      (bind _hitcomponent_2 (Variables|Components|GetHitComponent)
        (:then
          (return (LocalVariables|GetbLocalFound) (Transformation|GetWorldTransform _hitcomponent_2)))
        (:else
          (return (LocalVariables|GetbLocalFound) ""))))))

(fn ChangeBuildStructure
  (bind _buildpreview (Variables|Default|GetBuildPreview)
    (:then
      (Actor|DestroyActor _buildpreview))
    (:else
      _))
  (CallFunction|SpawnBuildPreview (Variables|Default|GetStructureDebug)))

(fn IsBuildFloating
  (bind _buildtransform (Variables|Default|GetBuildTransform))
  (bind _returnvalue (Collision|LineTraceByChannel (.location _buildtransform) (- (.location _buildtransform) "0.000000,0.000000,50.000000") "TraceTypeQuery1" false (Utilities|Array|MakeArray (Variables|Default|GetBuildPreview)) "None"))
  (return _returnvalue))

(fn IsBuildonFoundation
  (bind _buildpreview (Variables|Default|GetBuildPreview))
  (bind _staticmesh (Variables|/Game/Blueprints/BuildingSystem/BP_BuildableMaster.BP_BuildableMaster_C|GetStaticMesh _buildpreview))
  (bind _returnvalue (Transformation|GetWorldLocation _staticmesh))
  (bind (_outhit _returnvalue_2) (Collision|LineTraceByChannel _returnvalue (- _returnvalue "0.000000,0.000000,50.000000") "TraceTypeQuery1" false (Utilities|Array|MakeArray (Variables|Default|GetBuildPreview)) "None"))
  (if _returnvalue_2
    (return (Actor|ActorHasTag (.HitActor (Collision|BreakHitResult _outhit)) "Foundation"))
    (else
      (return false))))