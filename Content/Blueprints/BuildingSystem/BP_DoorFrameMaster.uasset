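; BP_DoorFrameMaster is the master Blueprint for door frame pieces in the building system.
; GetBoxes returns its attachment boxes: one door, two ceiling, two triangle ceiling, four torch and one wall, apparently as sockets for placing other pieces.
; It has no active logic of its own beyond that list, as the event stubs are disabled and the construction script only calls the parent.
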(event EventBeginPlay
  (|CallParentFunction) ; This node is disabled and will not be called.\nDrag off pins to build functionality.
)

(event Collision|EventActorBeginOverlap
  (params (OtherActor :type Actor%20Object%20Reference))
  (|CallParentFunction OtherActor) ; This node is disabled and will not be called.\nDrag off pins to build functionality.
)

(event EventTick
  (params (DeltaSeconds :type Float%20%28single-precision%29))
  (|CallParentFunction DeltaSeconds) ; This node is disabled and will not be called.\nDrag off pins to build functionality.
)

(fn ConstructionScript
  (|CallParentFunction))

(fn GetBoxes
  (return (Utilities|Array|MakeArray (Variables|Default|GetDoorBox) (Variables|Default|GetCeiling) (Variables|Default|GetCeiling1) (Variables|Default|GetTriangleCeiling) (Variables|Default|GetTriangleCeiling1) (Variables|Default|GetTorchBox3) (Variables|Default|GetTorchBox1) (Variables|Default|GetTorchBox) (Variables|Default|GetTorchBox2) (Variables|Default|GetWall))))