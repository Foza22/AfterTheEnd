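; Base third-person hatchet that chops harvestable large items and damages other actors.
; UseItem plays chop montages; Notify passes the owner's arrow transform to ServerOverlap for a sphere overlap, with damage reduced by character armor.
; Large items lose health, granting DataTable resources scaled by damage, tool type, tier and randomness, or get replaced by a destruct actor at zero health.
; HitFXMulticast spawns impact particles and sound for large-item hits.
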(event Custom|GetRotationClient
  (bind (_location _rotation) (Class|BPICharacter|GetArrowLocation(Message) (Components|GetOwner)))
  (CallFunction|ServerOverlap _location _rotation))

(event Custom|ServerOverlap
  (params (SpherePos :type Vector) (SphereRot :type Rotator))
  (bind (_outactors _returnvalue) (Collision|SphereOverlapActors SpherePos 4e+01 (Utilities|Array|MakeArray "ObjectTypeQuery7" "ObjectTypeQuery3") 0 (Utilities|Array|MakeArray (Variables|Default|GetCharacter%20Ref))))
  (if _returnvalue
    (for _array_element _outactors
      (bind _finaldamage (CallFunction|CalculateDamage _array_element (Math|Conversions|ToFloat(Integer) (Utilities|Struct|BreakS_ItemInfo (Variables|Default|GetItemInfo)))))
      (if (Utilities|DoesObjectImplementInterface _array_element "/Game/Blueprints/Interfaces/BPI_LargeItem.BPI_LargeItem_C")
        (CallFunction|HarvestFoliage _finaldamage _array_element)
        (CallFunction|HitFXMulticast SpherePos SphereRot)
        (else
          (Game|Damage|ApplyDamage _array_element _finaldamage (Pawn|GetController (Variables|Default|GetCharacter%20Ref)) self "/Script/Engine.DamageType"))))))

(event Custom|HitFXMulticast
  (params (Location :type Vector) (Rotation :type Rotator))
  (bind _outhit (Collision|LineTraceByChannel Location (* (Math|Vector|GetForwardVector Rotation) (Variables|Default|GetTraceDistance)) "TraceTypeQuery2" false 0 "None"))
  (Effects|SpawnEmitteratLocation (Variables|Default|GetHitEffect) (.ImpactPoint (Collision|BreakHitResult _outhit)))
  (Audio|PlaySoundatLocation (Variables|Default|GetHitSound) (.ImpactPoint (Collision|BreakHitResult _outhit)) "0, 0, 0" 1.0 1.0 0.0 "/Game/Assets/Sounds/Harvesting/RockSFX/ATT_Harvesting.ATT_Harvesting" 0 0 0))

(event EventBeginPlay
  (|CallParentFunction) ; This node is disabled and will not be called.\nDrag off pins to build functionality.
)

(event Collision|EventActorBeginOverlap
  (params (OtherActor :type Actor%20Object%20Reference))
  (|CallParentFunction OtherActor) ; This node is disabled and will not be called.\nDrag off pins to build functionality.
)

(event EventTick
  (params (DeltaSeconds :type Float%20%28single-precision%29))
  (|CallParentFunction DeltaSeconds) ; This node is disabled and will not be called.\nDrag off pins to build functionality.
)

(event EventUseItem
  (params (CharacterRef :type BP%20Base%20Character%20Object%20Reference))
  (if (not (Variables|Default|GetIsSwinging))
    (Variables|Default|SetIsSwinging true)
    (bind _output_get (Variables|Default|SetCharacter%20Ref CharacterRef))
    (Class|BPICharacter|FPMontage(Message) _output_get "/Game/Assets/Man/Animations/Montages/AM_Hatchet_Chop.AM_Hatchet_Chop")
    (Class|BPICharacter|TPMontage(Message) _output_get "/Game/Assets/Man/Animations/Montages/AM_Hatchet_Chop.AM_Hatchet_Chop")))

(event EventNotify
  (CallFunction|GetRotationClient))

(event EventEndAnimation
  (Variables|Default|SetIsSwinging false))

(fn ConstructionScript
  (|CallParentFunction))

(fn HarvestFoliage
  (params (Damage :type Float%20%28double-precision%29) (Ref :type Actor%20Object%20Reference))
  (LocalVariables|SetLocalDamage Damage)
  (bind _itemref (Class|BPILargeItem|GetItemRef(Message) Ref))
  (Utilities|IsValid _itemref
    (:Is%20Valid
      (LocalVariables|SetLocalHealth (- (Variables|/Game/Blueprints/HarvestingSystem/BP_LargeItemMaster.BP_LargeItemMaster_C|GetHealth _itemref) (LocalVariables|GetLocalDamage)))
      (if (<= (LocalVariables|GetLocalHealth) 0.0)
        (bind _returnvalue (Utilities|GetDataTableRow "/Game/Blueprints/DataTables/DT_LargetItemResources.DT_LargetItemResources" (Utilities|String|StringToName (Utilities|GetClassDisplayName (Utilities|GetClass _itemref))))
          (:then
            (LocalVariables|SetDestructClass (.Class (Utilities|Struct|BreakS_LargeItem _returnvalue)))
            (LocalVariables|SetLocalTransform (Transformation|GetActorTransform _itemref))
            (Actor|DestroyActor _itemref)
            (Game|SpawnActorfromClass (LocalVariables|GetDestructClass) (LocalVariables|GetLocalTransform) "Undefined" 0 (Transformation|GetActorForwardVector (Variables|Default|GetCharacter%20Ref)) 0)))
        (else
          (Variables|/Game/Blueprints/HarvestingSystem/BP_LargeItemMaster.BP_LargeItemMaster_C|SetHealth _itemref (LocalVariables|GetLocalHealth))
          (bind _returnvalue_2 (Utilities|GetDataTableRow "/Game/Blueprints/DataTables/DT_LargetItemResources.DT_LargetItemResources" (Utilities|String|StringToName (Utilities|GetClassDisplayName (Utilities|GetClass _itemref))))
            (:then
              (bind _output_get (LocalVariables|SetGivenResources (.GivenItems (Utilities|Struct|BreakS_LargeItem _returnvalue_2))))
              (for _array_element _output_get
                (if (not (<= (Math|Float|Truncate (|((((BaseVar*RateVar)*ToolTypeVar)*ToolTierVar)*DamageVar) (Math|Conversions|ToFloat(Integer) (.Quantity (Utilities|Struct|BreakS_ResourceStructure _array_element))) 1.0 (LocalVariables|GetLocalDamage) (Math|Float|SelectFloat (Math|Random|RandomFloatinRange 0.2 0.4) (Math|Random|RandomFloatinRange 0.01 0.1) (Utilities|Enum|Equal(Enum) (.PrefferedToolType (Utilities|Struct|BreakS_ResourceStructure _array_element)) (Variables|Default|GetToolType))) (Utilities|Select :Index (Variables|Default|GetToolTier) :NewEnumerator0 (Math|Random|RandomFloatinRange 0.8 1.2) :NewEnumerator1 (Math|Random|RandomFloatinRange 1.2 1.6)))) 0))
                  (bind _characterref (Class|BPICharacter|GetCharacterRef(Message) (Variables|Default|GetCharacter%20Ref)))
                  (Default|HarvestItemonServer _characterref (Utilities|Struct|MakeS_ResourceStructure (.ResourceName (Utilities|Struct|BreakS_ResourceStructure _array_element)) (Math|Float|Truncate (|((((BaseVar*RateVar)*ToolTypeVar)*ToolTierVar)*DamageVar) (Math|Conversions|ToFloat(Integer) (.Quantity (Utilities|Struct|BreakS_ResourceStructure _array_element))) 1.0 (LocalVariables|GetLocalDamage) (Math|Float|SelectFloat (Math|Random|RandomFloatinRange 0.2 0.4) (Math|Random|RandomFloatinRange 0.01 0.1) (Utilities|Enum|Equal(Enum) (.PrefferedToolType (Utilities|Struct|BreakS_ResourceStructure _array_element)) (Variables|Default|GetToolType))) (Utilities|Select :Index (Variables|Default|GetToolTier) :NewEnumerator0 (Math|Random|RandomFloatinRange 0.8 1.2) :NewEnumerator1 (Math|Random|RandomFloatinRange 1.2 1.6)))) (.PrefferedToolType (Utilities|Struct|BreakS_ResourceStructure _array_element)))))))))))))

(fn CalculateDamage
  (params (HitActor :type Actor%20Object%20Reference) (BaseDamage :type Float%20%28double-precision%29))
  (LocalVariables|SetLocalDamage (* BaseDamage (Variables|Default|GetDamageMultiplier)))
  (if (Utilities|DoesObjectImplementInterface HitActor "/Game/Blueprints/Interfaces/BPI_Character.BPI_Character_C")
    (bind _amount (Class|BPICharacter|GetTotalArmorPieces(Message) HitActor))
    (switch int _amount
      (:0
        (return (* (LocalVariables|GetLocalDamage) 4.0)))
      (:1
        (return (* (LocalVariables|GetLocalDamage) 3.5)))
      (:2
        (return (* (LocalVariables|GetLocalDamage) 3.0)))
      (:3
        (return (* (LocalVariables|GetLocalDamage) 2.5)))
      (:4
        (return (* (LocalVariables|GetLocalDamage) 2.0))))
    (else
      (return (* (LocalVariables|GetLocalDamage) 4.0)))))