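; Third-person base hatchet tool that plays chop montages and harvests large foliage resources such as trees.
; An anim notify gets the owner's arrow location and runs a server sphere overlap around it, with a debug sphere drawn.
; Each hit loses health; surviving targets yield items from DT_LargetItemResources, keyed by class name.
; Depleted targets are swapped for that row's destructible class, spawned along the character's forward vector.
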(event Custom|GetRotationClient
  (bind _location (Class|BPICharacter|GetArrowLocation(Message) (Components|GetOwner)))
  (CallFunction|ServerOverlap _location))

(event Custom|ServerOverlap
  (params (SpherePos :type Vector))
  (bind (_outactors _returnvalue) (Collision|SphereOverlapActors SpherePos 4e+01 (Utilities|Array|MakeArray "ObjectTypeQuery7") 0 (Utilities|Array|MakeArray (Variables|Default|GetCharacter%20Ref))))
  (Rendering|Debug|DrawDebugSphere SpherePos 4e+01 12 "(R=1.000000,G=1.000000,B=1.000000,A=1.000000)" 2.0 1.0)
  (if _returnvalue
    (for _array_element _outactors
      (CallFunction|HarvestFoliage 15.0 _array_element))))

(event EventBeginPlay
  (|CallParentFunction) ; This node is disabled and will not be called.\nDrag off pins to build functionality.
)

(event Collision|EventActorBeginOverlap
  (params (OtherActor :type Actor%20Object%20Reference))
  (|CallParentFunction OtherActor) ; This node is disabled and will not be called.\nDrag off pins to build functionality.
)

(event EventTick
  (params (DeltaSeconds :type Float%20%28single-precision%29))
  (|CallParentFunction DeltaSeconds) ; This node is disabled and will not be called.\nDrag off pins to build functionality.
)

(event EventUseItem
  (params (CharacterRef :type BP%20Base%20Character%20Object%20Reference))
  (if (not (Variables|Default|GetIsSwinging))
    (Variables|Default|SetIsSwinging true)
    (bind _output_get (Variables|Default|SetCharacter%20Ref CharacterRef))
    (Class|BPICharacter|FPMontage(Message) _output_get "/Game/Assets/Man/Animations/Montages/AM_Hatchet_Chop.AM_Hatchet_Chop")
    (Class|BPICharacter|TPMontage(Message) _output_get "/Game/Assets/Man/Animations/Montages/AM_Hatchet_Chop.AM_Hatchet_Chop")))

(event EventNotify
  (CallFunction|GetRotationClient))

(event EventEndAnimation
  (Variables|Default|SetIsSwinging false))

(fn ConstructionScript
  (|CallParentFunction))

(fn HarvestFoliage
  (params (Damage :type Float%20%28double-precision%29) (Ref :type Actor%20Object%20Reference))
  (LocalVariables|SetLocalDamage Damage)
  (bind _itemref (Class|BPILargeItem|GetItemRef(Message) Ref))
  (Utilities|IsValid _itemref
    (:Is%20Valid
      (LocalVariables|SetLocalHealth (- (Variables|/Game/HarvestingSystem/BP_LargeItemMaster.BP_LargeItemMaster_C|GetHealth _itemref) (LocalVariables|GetLocalDamage)))
      (if (<= (LocalVariables|GetLocalHealth) 0.0)
        (bind _returnvalue (Utilities|GetDataTableRow "/Game/Blueprints/DataTables/DT_LargetItemResources.DT_LargetItemResources" (Utilities|String|StringToName (Utilities|GetClassDisplayName (Utilities|GetClass _itemref))))
          (:then
            (LocalVariables|SetDestructClass (.Class (Utilities|Struct|BreakS_LargeItem _returnvalue)))
            (LocalVariables|SetLocalTransform (Transformation|GetActorTransform _itemref))
            (Actor|DestroyActor _itemref)
            (Game|SpawnActorfromClass (LocalVariables|GetDestructClass) (LocalVariables|GetLocalTransform) "Undefined" 0 (Transformation|GetActorForwardVector (Variables|Default|GetCharacter%20Ref)) 0)))
        (else
          (Variables|/Game/HarvestingSystem/BP_LargeItemMaster.BP_LargeItemMaster_C|SetHealth _itemref (LocalVariables|GetLocalHealth))
          (bind _returnvalue_2 (Utilities|GetDataTableRow "/Game/Blueprints/DataTables/DT_LargetItemResources.DT_LargetItemResources" (Utilities|String|StringToName (Utilities|GetClassDisplayName (Utilities|GetClass _itemref))))
            (:then
              (bind _output_get (LocalVariables|SetGivenResources (.GivenItems (Utilities|Struct|BreakS_LargeItem _returnvalue_2))))
              (for _array_element _output_get
                (bind _characterref (Class|BPICharacter|GetCharacterRef(Message) (Variables|Default|GetCharacter%20Ref)))
                (Default|HarvestItemonServer _characterref _array_element)))))))))