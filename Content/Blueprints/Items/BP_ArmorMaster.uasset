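; BP_ArmorMaster is the base Blueprint for armor items, with a skeletal mesh that follows a character's animation.
; Its construction script runs the parent's, then fills ItemInfo from the DT_Items row named by DataTableRowName.
; MasterPoseEvent gets the character's mesh through GetCharacterRefMessage and sets it as the armor mesh's leader pose component.
; GetArmorRef returns the armor instance itself.
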(event Custom|MasterPoseEvent
  (params (CharRef :type BP%20Base%20Character%20Object%20Reference))
  (bind _characterref (Class|BPICharacter|GetCharacterRef(Message) CharRef))
  (Components|SkinnedMesh|SetLeaderPoseComponent (Variables|Default|GetSkeletalMesh) (Variables|/Script/Engine.Character|GetMesh _characterref) false false))

(fn ConstructionScript
  (|CallParentFunction)
  (bind _returnvalue (Utilities|GetDataTableRow "/Game/Blueprints/DataTables/DT_Items.DT_Items" (Variables|Default|GetDataTableRowName))
    (:then
      (Variables|Default|SetItemInfo _returnvalue))))

(fn GetArmorRef
  (return self))